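; UFO character or pawn Blueprint that sets up its AI behavior through an AI controller.
; InitBlackBoard applies the UFOData blackboard, seeds NextLocation with the actor's current location, then runs the UFOTree behavior tree.
; An unconnected debug loop would print socket locations for the bone names in BonesName; BeginPlay and Tick do nothing.
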(event `self.ReceiveBeginPlay`)

(event `self.InitBlackBoard`
  (bind _asaicontroller (cast `AIController` (`self.GetController`)))
  (bind _blackboardcomponent (`AIController.UseBlackboard` _asaicontroller "/Game/Trees/UFOData.UFOData"))
  (`BlackboardComponent.SetValueAsVector` _blackboardcomponent "NextLocation" (`self.K2_GetActorLocation`))
  (`AIController.RunBehaviorTree` _asaicontroller "/Game/Trees/UFOTree.UFOTree"))

(fn `UserConstructionScript`)